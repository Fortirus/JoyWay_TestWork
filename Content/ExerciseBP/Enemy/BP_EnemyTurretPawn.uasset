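; Turret enemy pawn that turns its head toward a target, fires projectiles at the player and explodes on death.
; EnemyController handles attack cooldown and damage/death checks, while the pawn exposes EnemyInfo stats through getters.
; Attacks play a particle effect, then after a delay spawn a projectile aimed above the player's origin.
; RotateTo turns the head at constant speed and reports near-alignment using a signed sum of rotation deltas.
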(event `self.ReceiveBeginPlay`
  (setmembers `/Game/ExerciseBP/Enemy/struct_EnemyInfo` :`StructRef` (`self.EnemyInfo`) :`ThisEnemyController` (cast `/Game/ExerciseBP/Enemy/EnemyController` (`self.GetController`) :!pure true))
  (set `self.HeadRotationOffset` (`SceneComponent.RelativeRotation` (`self.HeadSkeletalMesh`))))

(event `/Game/ExerciseBP/bpi_Enemy.actionAttack`
  (bind ((`AttackDelay_4_A2D4A7A74916AA8F1C35818094DFDFE7` _attackdelay) (`AttackProjDamage_30_53D4DED745FAC3E02BBB1C83C0EC7E21` _attackprojdamage) (`AttackProjectileClass_23_D8E4E2CC4E7C86AA0C292988F6E01B3E` _attackprojectileclass)) (break `/Game/ExerciseBP/Enemy/struct_EnemyInfo` (`self.EnemyInfo`)))
  (bind ((`ThisEnemyController_21_A976C4384B5D609B37DC9997D14D96FB` _thisenemycontroller)) (break `/Game/ExerciseBP/Enemy/struct_EnemyInfo` (`self.EnemyInfo`)))
  (bind _returnvalue_location (`KismetMathLibrary.BreakTransform` (`SceneComponent.K2_GetComponentToWorld` (`self.ProjSpawnPoint`))))
  ;[1 1 1] Attacking
  (`/Game/ExerciseBP/Enemy/EnemyController.eAttackCooldown` _thisenemycontroller)
  (`ActorComponent.SetActive` (`self.PS_AttackSpawn`) true false) ; Activate Particle System for attack move
  (`KismetSystemLibrary.Delay` _attackdelay)
  (`|SpawnActorFromClass` _attackprojectileclass (`KismetMathLibrary.MakeTransform` _returnvalue_location (`KismetMathLibrary.FindLookAtRotation` _returnvalue_location (+ (`self.K2_GetActorLocation` (`/Game/ExerciseBP/Enemy/EnemyController.TargetPlayerActor` _thisenemycontroller)) (0.0 0.0 50.0)))) "Undefined" "OverrideRootScale" null _attackprojdamage null))

(event `/Game/ExerciseBP/bpi_Enemy.takeDamage`
  (params (damageAmount :type Integer) (fromActor :type "Actor Object Reference"))
  ;[1 1 1] Getting Damage
  (`/Game/ExerciseBP/Enemy/EnemyController.eTakeDamageAndCheckDie` (`.ThisEnemyController_21_A976C4384B5D609B37DC9997D14D96FB` (break `/Game/ExerciseBP/Enemy/struct_EnemyInfo` (`self.EnemyInfo`))) damageAmount))

(event `/Game/ExerciseBP/bpi_Enemy.actionDie`
  ;[1 1 1] Dying
  (`PrimitiveComponent.SetCollisionEnabled` (`self.CollisionCapsule`) "NoCollision")
  (bind _returnvalue (`GameplayStatics.SpawnEmitterAtLocation` "/Game/VFX/Particlse/ps_GrenadeExplosion.ps_GrenadeExplosion" (`SceneComponent.K2_GetComponentLocation` (`self.HeadSkeletalMesh`))))
  (`KismetSystemLibrary.Delay` 1.0)
  (`ActorComponent.K2_DestroyComponent` _returnvalue))

(fn `getAttackCD`
  (returns (AttackCD :type "Float (double-precision)"))
  (return (`.AttackCD_2_82B36921473410847A40938AE4A52785` (break `/Game/ExerciseBP/Enemy/struct_EnemyInfo` (`self.EnemyInfo`)))))

(fn `getDropRate`
  (returns (DropRate :type Integer))
  (return (`.DropRate_14_0C1F8E3D4211D92E94DF14AAE0F9F5ED` (break `/Game/ExerciseBP/Enemy/struct_EnemyInfo` (`self.EnemyInfo`)))))

(fn `getGameplayTags`
  (returns (actorGameplayTags :type "GameplayTagContainer Structure"))
  (return (`.GameplayTags_18_064DD7994AB00A1D6F3D15AF7EE715D7` (break `/Game/ExerciseBP/Enemy/struct_EnemyInfo` (`self.EnemyInfo`)))))

(fn `getSpawnHP`
  (returns (SpawnHP :type Integer))
  (return (`.SpawnHP_12_D1FE92004F28E7D453F9FAAAB6092B67` (break `/Game/ExerciseBP/Enemy/struct_EnemyInfo` (`self.EnemyInfo`)))))

(fn `rotateTo`
  (params (TargetLocation :type "Vector Structure") (DeltaTime :type "Float (double-precision)"))
  (returns (FinishRotation :type Boolean))
  (locals (TargetRotation :type "Rotator Structure" :default (struct)))
  (bind _headskeletalmesh (`self.HeadSkeletalMesh`))
  (bind _returnvalue (`SceneComponent.K2_GetComponentRotation` _headskeletalmesh))
  (bind _output_get (set `local.TargetRotation` (`KismetMathLibrary.ComposeRotators` (`KismetMathLibrary.FindLookAtRotation` (`SceneComponent.K2_GetComponentLocation` _headskeletalmesh) (+ TargetLocation (0.0 0.0 50.0))) (`self.HeadRotationOffset`))))
  (`SceneComponent.K2_SetWorldRotation` _headskeletalmesh (`KismetMathLibrary.RInterpTo_Constant` _returnvalue _output_get DeltaTime 100.0) false false)
  (bind (_returnvalue_roll _returnvalue_pitch _returnvalue_yaw) (`KismetMathLibrary.BreakRotator` (`KismetMathLibrary.NormalizedDeltaRotator` _returnvalue _output_get)))
  (return (< (+ _returnvalue_roll _returnvalue_pitch _returnvalue_yaw) 40.0)))

(fn `UserConstructionScript`)