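; Enemy character Blueprint that fires projectiles at the player and ragdolls on death, with its stats held in an EnemyInfo struct exposed through getters.
; Its EnemyController handles damage, death checks and attack cooldown.
; Attacks pass a DoIfAlive macro, activate particles, then spawn a delayed projectile rotated toward the target player.
; Death disables capsule collision and launches the physics mesh using the damaging actor's direction, or the last projectile hit normal as fallback.
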(event `self.ReceiveBeginPlay`
  (setmembers `/Game/ExerciseBP/Enemy/struct_EnemyInfo` :`StructRef` (`self.EnemyInfo`) :`ThisEnemyController` (cast `/Game/ExerciseBP/Enemy/EnemyController` (`self.GetController`) :!pure true)))

(event `self.Mesh.OnComponentHit`
  (params (HitComponent :type "PrimitiveComponent Object Reference") (OtherActor :type "Actor Object Reference") (OtherComp :type "PrimitiveComponent Object Reference") (NormalImpulse :type "Vector Structure") (Hit :type "HitResult Structure (by ref)"))
  ;[1 1 1] Getting Hit by Player Projectile
  (if (`KismetMathLibrary.ClassIsChildOf` (`GameplayStatics.GetObjectClass` OtherActor) "/Game/ExerciseBP/Guns/Base/BP_PlayerProjectileBase.BP_PlayerProjectileBase_C")
    (set `self.LastHitLock` (`.ImpactNormal` (`GameplayStatics.BreakHitResult` Hit)))))

(event `/Game/ExerciseBP/bpi_Enemy.actionAttack`
  (bind ((`AttackDelay_4_A2D4A7A74916AA8F1C35818094DFDFE7` _attackdelay) (`AttackProjDamage_30_53D4DED745FAC3E02BBB1C83C0EC7E21` _attackprojdamage) (`AttackProjectileClass_23_D8E4E2CC4E7C86AA0C292988F6E01B3E` _attackprojectileclass)) (break `/Game/ExerciseBP/Enemy/struct_EnemyInfo` (`self.EnemyInfo`)))
  (bind ((`ThisEnemyController_21_A976C4384B5D609B37DC9997D14D96FB` _thisenemycontroller)) (break `/Game/ExerciseBP/Enemy/struct_EnemyInfo` (`self.EnemyInfo`)))
  (bind _returnvalue_location (`KismetMathLibrary.BreakTransform` (`SceneComponent.K2_GetComponentToWorld` (`self.ProjSpawnPoint`))))
  ;[1 1 1] Attacking
  (`self.DoIfAlive`
    (:`Out`
      (`/Game/ExerciseBP/Enemy/EnemyController.eAttackCooldown` _thisenemycontroller)
      (`ActorComponent.SetActive` (`self.PS_AttackSpawn`) true false) ; Activate Particle System for attack move
      (`KismetSystemLibrary.Delay` _attackdelay)
      (`|SpawnActorFromClass` _attackprojectileclass (`KismetMathLibrary.MakeTransform` _returnvalue_location (`KismetMathLibrary.FindLookAtRotation` _returnvalue_location (+ (`self.K2_GetActorLocation` (`/Game/ExerciseBP/Enemy/EnemyController.TargetPlayerActor` _thisenemycontroller)) (0.0 0.0 50.0)))) "Undefined" "OverrideRootScale" null _attackprojdamage null))))

(event `/Game/ExerciseBP/bpi_Enemy.takeDamage`
  (params (damageAmount :type Integer) (fromActor :type "Actor Object Reference"))
  ;[1 1 1] Getting Damage
  (set `self.DamageActor` fromActor)
  (`/Game/ExerciseBP/Enemy/EnemyController.eTakeDamageAndCheckDie` (`.ThisEnemyController_21_A976C4384B5D609B37DC9997D14D96FB` (break `/Game/ExerciseBP/Enemy/struct_EnemyInfo` (`self.EnemyInfo`))) damageAmount))

(event `/Game/ExerciseBP/bpi_Enemy.actionDie`
  (bind _mesh (`self.Mesh`))
  ;[1 1 1] Dying
  (`PrimitiveComponent.SetCollisionEnabled` (`self.CapsuleComponent`) "NoCollision")
  (`PrimitiveComponent.SetSimulatePhysics` _mesh true)
  (bind _damageactor (`self.DamageActor`)
    (:`then`
      (bind _returnvalue (`FunctionLibrary_Exercise.VectorFormToActor` self (0.0 0.0 50.0) _damageactor))
      (`PrimitiveComponent.AddImpulse` _mesh (* _returnvalue -3000) "None" true) ; if an actor that was the cause of the death is specified - an impulse from him
    )
    (:`else`
      (`PrimitiveComponent.AddImpulse` _mesh (* (`self.LastHitLock`) 3000) "None" true) ; if not - form the last hit location
    )))

(fn `getAttackCD`
  (returns (AttackCD :type "Float (double-precision)"))
  (return (`.AttackCD_2_82B36921473410847A40938AE4A52785` (break `/Game/ExerciseBP/Enemy/struct_EnemyInfo` (`self.EnemyInfo`)))))

(fn `getDropRate`
  (returns (DropRate :type Integer))
  (return (`.DropRate_14_0C1F8E3D4211D92E94DF14AAE0F9F5ED` (break `/Game/ExerciseBP/Enemy/struct_EnemyInfo` (`self.EnemyInfo`)))))

(fn `getGameplayTags`
  (returns (actorGameplayTags :type "GameplayTagContainer Structure"))
  (return (`.GameplayTags_18_064DD7994AB00A1D6F3D15AF7EE715D7` (break `/Game/ExerciseBP/Enemy/struct_EnemyInfo` (`self.EnemyInfo`)))))

(fn `getSpawnHP`
  (returns (SpawnHP :type Integer))
  (return (`.SpawnHP_12_D1FE92004F28E7D453F9FAAAB6092B67` (break `/Game/ExerciseBP/Enemy/struct_EnemyInfo` (`self.EnemyInfo`)))))

(fn `UserConstructionScript`)