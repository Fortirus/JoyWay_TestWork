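; Physics-driven pickup item for health and ammo packs, which flies to the player's camera when taken and is added to the inventory.
; Construction sets color and icon from ItemType, using a palette DataTable and layered-material parameters on the VFX plane.
; The camera-facing VFX fades in after a landing delay.
; Take disables physics and collision, then a timeline drives the fade and flight before calling the controller and destroying the actor.
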(event `self.ReceiveBeginPlay`
  (bind _vfxplane (`self.vfxPlane`))
  (`|ExecutionSequence`
    (:`then_0`
      (`SceneComponent.SetVisibility` (`self.vfxPlane`) false false)
      (`/Engine/EditorBlueprintResources/StandardMacros.IsValid` (`self.playerCamera`)
        (:`Is Valid`
          (`self.SetActorTickEnabled` true))
        (:`Is Not Valid`
          (`KismetSystemLibrary.Delay` 0.0) ; if it's start of the game, we need to wait to spawn of the player character
          (bind _playercamera (message `/Game/ExerciseBP/bpi_Player.getPlayerCamera` (`GameplayStatics.GetPlayerPawn` 0)))
          (set `self.playerCamera` _playercamera)
          (`self.SetActorTickEnabled` true))))
    (:`then_1`
      (`KismetSystemLibrary.Delay` 1.5) ; Delay about when it hits the floor
      (`/Engine/EditorBlueprintResources/StandardMacros.IsValid` self
        (:`Is Valid`
          (`SceneComponent.SetVisibility` _vfxplane true false)
          (bind (_direction _opacityparam) (`Timeline|TimelineFadeIn` :!via `PlayFromStart` :!label _label)
            (:`Update`
              (`MeshComponent.SetScalarParameterValueOnMaterials` _vfxplane "blAllOpacityMultiply" _opacityparam) ; Change VFX Place visability
            )))))))

(event `/Game/ExerciseBP/Items/bpi_LevelItem.Take`
  (params (tagetPlayerController :type "/Game/ExerciseBP/PCandVR_PlayerController Object Reference"))
  (bind _mainmesh (`self.mainMesh`))
  (set `self.PlayerPCVRController` tagetPlayerController)
  (set `self.isPicked` true)
  (`PrimitiveComponent.SetSimulatePhysics` _mainmesh false)
  (`PrimitiveComponent.SetEnableGravity` _mainmesh false)
  (`PrimitiveComponent.SetCollisionEnabled` _mainmesh "NoCollision")
  (`|ExecutionSequence`
    (:`then_0`
      (goto _label :!via `Stop`))
    (:`then_1`
      (bind (_direction _opacityparam _lockalpha) (`Timeline|TimelineFadeAndGo` :!via `PlayFromStart`)
        (:`Update`
          (`MeshComponent.SetScalarParameterValueOnMaterials` (`self.vfxPlane`) "blAllOpacityMultiply" _opacityparam) ; Change VFX Place visability
          (`SceneComponent.K2_SetWorldLocation` (`self.mainMesh`) (`KismetMathLibrary.VLerp` (`SceneComponent.K2_GetComponentLocation` (`self.mainMesh`)) (- (`SceneComponent.K2_GetComponentLocation` (`self.playerCamera`)) (0.0 0.0 50.0)) _lockalpha) false false) ; SWEEP to camera location
        )
        (:`Finished`
          (`/Game/ExerciseBP/PCandVR_PlayerController.eAddInventoryItem` (`self.PlayerPCVRController`) (`self.itemType`))
          (`self.K2_DestroyActor`))))))

(event `self.ReceiveTick`
  (params (DeltaSeconds :type "Float (single-precision)"))
  (`SceneComponent.K2_SetWorldRotation` (`self.vfxScene`) (`KismetMathLibrary.FindLookAtRotation` (`SceneComponent.K2_GetComponentLocation` (`self.vfxScene`)) (`SceneComponent.K2_GetComponentLocation` (`self.playerCamera`))) false false) ; so it's ALWAYS face Player Camera
)

(event `eAddExtraMotion`
  (bind _mainmesh (`self.mainMesh`))
  (`PrimitiveComponent.SetPhysicsLinearVelocity` _mainmesh (* (`KismetMathLibrary.RandomUnitVector`) 250) false "None")
  (`PrimitiveComponent.SetAllPhysicsAngularVelocityInDegrees` _mainmesh (* (`KismetMathLibrary.RandomUnitVector`) 150) false))

(fn `getGameplayTags`
  (returns (actorGameplayTags :type "GameplayTagContainer Structure"))
  (return (`self.GameplayTags`)))

(fn `ItesIsReady`
  (returns (Yes :type Boolean))
  (return (not (`self.isPicked`))))

(fn `UserConstructionScript`
  (locals (fxMatereal :type "MaterialInterface Object Reference") (fxMaterealDI :type "MaterialInstanceDynamic Object Reference"))
  (bind _vfxplane (`self.vfxPlane`))
  (bind _maincolor (`self.mainColor`))
  (bind _fxmaterealdi (`local.fxMaterealDI`))
  (`|ExecutionSequence`
    (:`then_0`
      (switch `/Game/ExerciseBP/Items/eItemTypes` (`self.itemType`)
        (:`NewEnumerator0`
          ;[1 1 1] For HP packs
          (bind _returnvalue (`|GetDataTableRow` "/Game/ExerciseBP/Utility/dt_ColorsPalette.dt_ColorsPalette" "cLGreen")
            (:`then`
              (set `self.mainColor` (`.Color_12_D2C43DBD4B34A0ED29E2D6963CC129AB` (break `/Game/ExerciseBP/Utility/structure_ColorMap` _returnvalue)))
              (set `self.itemIcon` "/Game/Matereals/Textures/icon_HP_invert.icon_HP_invert"))))
        (:`NewEnumerator1`
          ;[1 1 1] For Ammunition
          (bind _returnvalue_2 (`|GetDataTableRow` "/Game/ExerciseBP/Utility/dt_ColorsPalette.dt_ColorsPalette" "cViolet")
            (:`then`
              (set `self.mainColor` (`.Color_12_D2C43DBD4B34A0ED29E2D6963CC129AB` (break `/Game/ExerciseBP/Utility/structure_ColorMap` _returnvalue_2)))
              (set `self.itemIcon` "/Game/Matereals/Textures/icon_AmmoBold.icon_AmmoBold"))))))
    (:`then_1`
      (`MeshComponent.SetVectorParameterValueOnMaterials` (`self.mainMesh`) "MainColor" (`KismetMathLibrary.Conv_LinearColorToVector` (`self.mainColor`)))
      (`MeshComponent.SetScalarParameterValueOnMaterials` _vfxplane "None" 0.0) ; Auto made material instance
      (bind _output_get (set `local.fxMatereal` (`PrimitiveComponent.GetMaterial` _vfxplane 0)))
      (bind _asmaterial_instance_dynamic (cast `MaterialInstanceDynamic` _output_get))
      (bind _output_get_2 (set `local.fxMaterealDI` _asmaterial_instance_dynamic))
      (`MaterialInstanceDynamic.SetVectorParameterValueByInfo` _output_get_2 (`MaterialInterface.GetParameterInfo` _fxmaterealdi "LayerParameter" "dl_BaseColor" "/Game/Matereals/Layers/ml_DynamicLines.ml_DynamicLines") _maincolor)
      (`MaterialInstanceDynamic.SetVectorParameterValueByInfo` _output_get_2 (`MaterialInterface.GetParameterInfo` _fxmaterealdi "LayerParameter" "ml_tColorMulti" "/Game/Matereals/Layers/ml_Texture.ml_Texture") _maincolor)
      (`MaterialInstanceDynamic.SetTextureParameterValueByInfo` _output_get_2 (`MaterialInterface.GetParameterInfo` _fxmaterealdi "LayerParameter" "ml_tTexture" "/Game/Matereals/Layers/ml_Texture.ml_Texture") (`self.itemIcon`)))))