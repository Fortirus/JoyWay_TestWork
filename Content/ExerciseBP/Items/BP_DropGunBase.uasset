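; Base actor for a dropped gun pickup that hands its gun to the player controller that takes it.
; The construction script previews GunClass through a child actor, which BeginPlay destroys and replaces with a spawned, attached gun actor.
; Take marks the pickup as picked, passes that same gun to the controller's EPickGun and destroys itself.
; Query functions expose its gameplay tags and whether it is still unpicked.
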(event `self.ReceiveBeginPlay`
  (`ActorComponent.K2_DestroyComponent` (`self.EditViewChildGunActor`))
  (bind _returnvalue (`|SpawnActorFromClass` (`self.GunClass`) (`KismetMathLibrary.MakeTransform` (0.0 0.0 0.0)) "Undefined" "OverrideRootScale" self null))
  (bind _output_get (set `self.GunActor` _returnvalue))
  (`self.K2_AttachToActor` _output_get self "None" "KeepRelative" "KeepRelative" "KeepRelative" true))

(event `/Game/ExerciseBP/Items/bpi_LevelItem.Take`
  (params (tagetPlayerController :type "/Game/ExerciseBP/PCandVR_PlayerController Object Reference"))
  (set `self.isPicked` true)
  (`/Game/ExerciseBP/PCandVR_PlayerController.ePickGun` tagetPlayerController (`self.GunActor`))
  (`self.K2_DestroyActor`))

(fn `getGameplayTags`
  (returns (actorGameplayTags :type "GameplayTagContainer Structure"))
  (return (`self.GameplayTags`)))

(fn `ItesIsReady`
  (returns (Yes :type Boolean))
  (return (not (`self.isPicked`))))

(fn `UserConstructionScript`
  (bind _gunclass (`self.GunClass`))
  (if (`KismetSystemLibrary.IsValidClass` _gunclass)
    (`ChildActorComponent.SetChildActorClass` (`self.EditViewChildGunActor`) _gunclass)))