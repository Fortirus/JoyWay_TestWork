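; Base gun Blueprint that spawns projectiles from a muzzle and tracks ammo.
; Construction attaches the muzzle arrow to the gun mesh's Muzzle socket, parents the muzzle component to it and fills ammo to max.
; Two fire functions aim at a target location or along muzzle rotation, each decrementing ammo once without checking it.
; Each spawns the per-round projectile count, combining aim with a random cone spread rotation per projectile.
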(fn `getSpreadRotation`
  (returns (ReturnValue :type "Rotator Structure"))
  (bind _spreaddegree (`self.SpreadDegree`))
  (if (< _spreaddegree 0.01)
    (return (`KismetMathLibrary.MakeRotator` 0.0))
    (else
      (return (`KismetMathLibrary.Conv_VectorToRotator` (`KismetMathLibrary.RandomUnitVectorInConeInDegrees` (1.0 0.0 0.0) _spreaddegree))))))

(fn `MainFireAtTargetLoc`
  (params (TargetLoc :type "Vector Structure"))
  (locals (fromMuzzleToTargetRot :type "Rotator Structure" :default (struct)) (newSpreadRotation :type "Rotator Structure" :default (struct)))
  (bind _returnvalue (`SceneComponent.K2_GetComponentLocation` (`self.Muzzle`)))
  (`/Engine/EditorBlueprintResources/StandardMacros.DecrementInt` (`self.CurAmmoCount`)
    (:`  `
      (set `local.fromMuzzleToTargetRot` (`KismetMathLibrary.FindLookAtRotation` _returnvalue TargetLoc))
      (for _ (range 1 (+ (`self.ProjPerRound`) 1))
        (bind _output_get (set `local.newSpreadRotation` (`self.getSpreadRotation`)))
        (`|SpawnActorFromClass` (`self.ProjectileClass`) (`KismetMathLibrary.MakeTransform` _returnvalue (`KismetMathLibrary.ComposeRotators` (`local.fromMuzzleToTargetRot`) _output_get)) "Undefined" "OverrideRootScale" null 10 null)))))

(fn `MainFireForward`
  (locals (newSpreadRotation :type "Rotator Structure" :default (struct)))
  (bind _muzzle (`self.Muzzle`))
  (`/Engine/EditorBlueprintResources/StandardMacros.DecrementInt` (`self.CurAmmoCount`)
    (:`  `
      (for _ (range 1 (+ (`self.ProjPerRound`) 1))
        (bind _output_get (set `local.newSpreadRotation` (`self.getSpreadRotation`)))
        (`|SpawnActorFromClass` (`self.ProjectileClass`) (`KismetMathLibrary.MakeTransform` (`SceneComponent.K2_GetComponentLocation` _muzzle) (`KismetMathLibrary.ComposeRotators` (`SceneComponent.K2_GetComponentRotation` _muzzle) _output_get)) "Undefined" "OverrideRootScale" null 10 null)))))

(fn `UserConstructionScript`
  (`SceneComponent.K2_AttachToComponent` (`self.MuzzleArrow`) (`self.GunMesh`) "Muzzle" "KeepRelative" "KeepRelative" "KeepRelative" true)
  (`SceneComponent.K2_AttachToComponent` (`self.Muzzle`) (`self.MuzzleArrow`) "Muzzle" "KeepRelative" "KeepRelative" "KeepRelative" true)
  (set `self.CurAmmoCount` (`self.MaxAmmoCount`)))